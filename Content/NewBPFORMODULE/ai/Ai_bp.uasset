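; Zombie AI character Blueprint that provides attack and walk behaviors.
; Attack plays a 2D sound and a one-shot animation, then immediately broadcasts OnAttackEnd, while Walk loops a walking animation; both print debug text.
; BeginPlay and Chase are empty, leaving the intended loop of walking to the player, attacking, pausing and chasing again disconnected, so it never runs.
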(event Custom|Chase)

(event Custom|Walk
  (Components|Animation|PlayAnimation (Variables|Character|GetMesh) "/Game/NewBPFORMODULE/ai/AnimFile/Walking__2_.Walking__2_" true)
  (Development|PrintString "Walk"))

(event Custom|attack
  (Audio|PlaySound2D "/Game/NewBPFORMODULE/ai/AnimFile/zombi-chuma-atakuet-chelovechestvo_Cue.zombi-chuma-atakuet-chelovechestvo_Cue" 1.0 1.0 0.0 0 0)
  (Components|Animation|PlayAnimation (Variables|Character|GetMesh) "/Game/NewBPFORMODULE/ai/AnimFile/Zombie_Attack__1_.Zombie_Attack__1_" false)
  (Development|PrintString "Attcak")
  (Default|CallOnAttackEnd))

(event EventBeginPlay)

(fn ConstructionScript)