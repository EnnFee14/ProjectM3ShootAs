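; Actor that plays an expanding radial scan effect through a decal with a dynamic material, driven by a settings struct.
; Begin sets up the material, attaches to or copies position and velocity from a target actor or component, and sets a lifespan.
; Each tick, an expansion curve drives decal scale and the material's Distance parameter, while inherited velocity drifts with drag.
; Optionally, the source's forward vector feeds the material as SourceDirection.
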(event EventTick
  (params (DeltaSeconds :type Float%20%28single-precision%29))
  (Utilities|FlowControl|Sequence
    (:then_0
      (if (.ParentSourceDirection (Utilities|Struct|BreakS_RadialScanSettings (Variables|Effect|GetSettings)))
        (Internal|UpdateSourceDirection)))
    (:then_1
      (Internal|UpdateRadialScan)
      (Transformation|AddActorWorldOffset (* (* (Variables|Default|GetVelocity) (.ParentVelocityScale (Utilities|Struct|BreakS_RadialScanSettings (Variables|Effect|GetSettings)))) (Utilities|Time|GetWorldDeltaSeconds)))
      (Variables|Default|SetVelocity (* (Variables|Default|GetVelocity) (- 1.0 (* (.VelocityDrag (Utilities|Struct|BreakS_RadialScanSettings (Variables|Effect|GetSettings))) (Utilities|Time|GetWorldDeltaSeconds))))))))

(fn ConstructionScript)

(fn SetScanMaterial
  (params (Material :type Material%20Interface%20Object%20Reference))
  (Utilities|IsValid Material
    (:Is%20Valid
      (bind _asmaterial_instance_dynamic (Utilities|Casting|CastToMaterialInstanceDynamic Material)
        (:then
          (Variables|Reference|SetMaterialInstance _asmaterial_instance_dynamic))
        (:CastFailed
          (bind _returnvalue (Rendering|Material|CreateDynamicMaterialInstance Material "None" "None" :!class /Script/Engine.KismetMaterialLibrary))
          (Variables|Reference|SetMaterialInstance _returnvalue)))
      (bind _materialinstance (Variables|Reference|GetMaterialInstance)
        (:then
          (Rendering|Components|Decal|SetDecalMaterial (Variables|Default|GetDecal) _materialinstance)
          (bind _returnvalue_2 (Rendering|Material|GetVectorParameterValue (Variables|Reference|GetMaterialInstance) "SphereScale" :!class /Script/Engine.MaterialInstanceDynamic))
          (Variables|Reference|SetSphereScale (Math|Conversions|ToVector(LinearColor) _returnvalue_2)))
        (:else)))))

(fn SetTargetActor
  (params (Target :type Actor%20Object%20Reference))
  (Variables|Reference|SetTargetActor Target)
  (Variables|Reference|SetTargetComponent 0)
  (bind _targetactor (Variables|Reference|GetTargetActor)
    (:then
      (if (!= _targetactor self)
        (if (.ParentSourcePosition (Utilities|Struct|BreakS_RadialScanSettings (Variables|Effect|GetSettings)))
          (Transformation|AttachActorToActor self (Variables|Reference|GetTargetActor) "None" "SnapToTarget" "SnapToTarget" "KeepRelative" true)
          (else
            (Transformation|SetActorLocation (Transformation|GetActorLocation (Variables|Reference|GetTargetActor)) false false)
            (Variables|Default|SetVelocity (Transformation|GetVelocity (Variables|Reference|GetTargetActor)))))))
    (:else)))

(fn SetTargetComponent
  (params (Target :type Scene%20Component%20Object%20Reference))
  (Variables|Reference|SetTargetComponent Target)
  (Variables|Reference|SetTargetActor 0)
  (bind _targetcomponent (Variables|Reference|GetTargetComponent)
    (:then
      (if (!= _targetcomponent (Variables|Default|GetDecal))
        (if (.ParentSourcePosition (Utilities|Struct|BreakS_RadialScanSettings (Variables|Effect|GetSettings)))
          (Transformation|AttachComponentToComponent (Variables|Reference|GetTargetComponent) "None" "SnapToTarget" "SnapToTarget" "KeepRelative" true)
          (else
            (Transformation|SetActorLocation (Transformation|GetWorldLocation (Variables|Reference|GetTargetComponent)) false false)
            (Variables|Default|SetVelocity (Transformation|GetVelocity (Components|GetOwner (Variables|Reference|GetTargetComponent))))))))
    (:else)))

(fn SetupReference
  (bind _targetactor (Variables|Reference|GetTargetActor)
    (:then
      (Reference|SetTargetActor _targetactor))
    (:else
      (bind _targetcomponent (Variables|Reference|GetTargetComponent)
        (:then
          (Reference|SetTargetComponent _targetcomponent))
        (:else
          (Reference|SetTargetActor self))))))

(fn UpdateSourceDirection
  (Utilities|IsValid (Variables|Reference|GetMaterialInstance)
    (:Is%20Valid
      (bind _targetactor (Variables|Reference|GetTargetActor)
        (:then
          (LocalVariables|SetSourceDirection (Transformation|GetActorForwardVector _targetactor)))
        (:else
          (bind _targetcomponent (Variables|Reference|GetTargetComponent)
            (:then
              (LocalVariables|SetSourceDirection (Math|Vector|GetForwardVector _targetcomponent)))
            (:else))))
      (Rendering|Material|SetVectorParameterValue (Variables|Reference|GetMaterialInstance) "SourceDirection" (Math|Conversions|ToLinearColor(Vector) (LocalVariables|GetSourceDirection)) :!class /Script/Engine.MaterialInstanceDynamic))))

(fn BeginRadialScan
  (Reference|SetScanMaterial (.Material (Utilities|Struct|BreakS_RadialScanSettings (Variables|Effect|GetSettings))))
  (Internal|SetupReference)
  (Internal|UpdateSourceDirection)
  (Actor|SetLifeSpan (.LifeTime (Utilities|Struct|BreakS_RadialScanSettings (Variables|Effect|GetSettings))))
  (Variables|Effect|SetStartTime (Utilities|Time|GetGameTimeinSeconds))
  (Variables|Effect|SetHasBegun true))

(fn UpdateRadialScan
  (bind _settings (Variables|Effect|GetSettings))
  (bind (_material _speed _lifetime _startoffset _parentsourceposition _parentsourcedirection _parentvelocityscale _velocitydrag _expansioncurve) (Utilities|Struct|BreakS_RadialScanSettings _settings))
  (if (Variables|Effect|GetHasBegun)
    (Variables|Effect|SetDistance (+ (* (Math|Curves|GetFloatValue _expansioncurve (/ (- (Utilities|Time|GetGameTimeinSeconds) (Variables|Effect|GetStartTime)) _lifetime)) (* _speed _lifetime)) _startoffset))
    (Transformation|SetRelativeScale3D (Variables|Default|GetDecal) (Math|Vector|VectorComponentMax "1.000000,1.000000,1.000000" (* (Variables|Reference|GetSphereScale) (* (Variables|Effect|GetDistance) 2.0))))
    (bind _materialinstance (Variables|Reference|GetMaterialInstance)
      (:then
        (Rendering|Material|SetScalarParameterValue _materialinstance "Distance" (Variables|Effect|GetDistance) :!class /Script/Engine.MaterialInstanceDynamic))
      (:else))))

(fn TestScan
  (Effect|BeginRadialScan)
  (Actor|SetLifeSpan 0.0))